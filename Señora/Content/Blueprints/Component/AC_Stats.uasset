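; Actor component that tracks health for its owner, handling damage and healing.
; A Damage event subtracts the absolute amount from HP, floored at zero, and calls the Died dispatcher when HP reaches zero.
; A Cure event raises HP up to MaxHP, with the healing function returning whether health is full.
; Both health functions print Spanish debug messages showing the resulting HP.
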(event `/Game/Blueprints/Interfaces/BPI_Stats.Damage`
  (params (Damage :type "Float (double-precision)") (Causer :type "Actor Object Reference") (Instigator :type "Controller Object Reference") (DamageType :type "DamageType Class Reference"))
  (bind _isdead (`self.takeDamage` Damage))
  (if _isdead
    (`self.Died`)))

(event `/Game/Blueprints/Interfaces/BPI_Stats.Cure`
  (params (CureAmount :type "Float (double-precision)"))
  (`self.Cure` CureAmount))

(fn `CureHealth`
  (params (CureAmount :type "Float (double-precision)"))
  (returns (isFull :type Boolean))
  ;[0 0.15 0.001821 0.502] Add Health
  (bind _output_get (set `self.HP` (`KismetMathLibrary.FMin` (+ CureAmount (`self.HP`)) (`self.MaxHP`))))
  (`KismetSystemLibrary.PrintString` (`KismetStringLibrary.Concat_StrStr` "Me cure ahora tengo " (`KismetStringLibrary.Conv_DoubleToString` _output_get) "de vida"))
  (return (== _output_get (`self.MaxHP`))))

(fn `takeDamage`
  (params (Damage :type "Float (double-precision)"))
  (returns (isDead :type Boolean))
  (bind _hp (`self.HP`))
  ;[0 0.15 0.001749 0.5] Substract HP
  (bind _output_get (set `self.HP` (`KismetMathLibrary.FMax` (- _hp (`KismetMathLibrary.Abs` Damage)))))
  (`KismetSystemLibrary.PrintString` (`KismetStringLibrary.Concat_StrStr` "Auch me hicieron " (`KismetStringLibrary.Conv_DoubleToString` Damage) " de daño y me quede con la siguiente vida" (`KismetStringLibrary.Conv_DoubleToString` _hp)) true true (struct :`G` 0.66 :`B` 1.0 :`A` 1.0) 10.0)
  ;[0.15 0 0 0.5] Return if is Dead
  (bind _output_get_2 (set `self.isDead` (== _output_get 0.0)))
  (return _output_get_2))
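; Player Blueprint that handles interaction, switching between default and fight-mode Enhanced Input contexts, and light punching.
; Interact messages the first actor in a list maintained through add and remove events.
; Light punch, gated by CanAttack, plays alternating montage sections, and SetCollision enables the matching left or right hit collider or disables both.
; Hits and the StatComponent's death event only print debug strings.
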(event `EnhancedInput|/Game/ThirdPerson/Input/Actions/IA_Interact`
  (params (ActionValue :type Boolean) (ElapsedSeconds :type "Float (double-precision)") (TriggeredSeconds :type "Float (double-precision)") (InputAction :type "InputAction Object Reference" :default "/Game/ThirdPerson/Input/Actions/IA_Interact.IA_Interact"))
  (bind _interactableitems (`self.InteractableItems`))
  ;[0.9115 0 0.832 0.5] Interaction System
  ;;[0 0.15 0.000323 0.5] Interact
  (:`Started`
    (if (`KismetArrayLibrary.Array_IsNotEmpty` _interactableitems)
      (message `/Game/Blueprints/Interfaces/BPI_Interactable.Interact` (`|GetArrayItem` _interactableitems) self))))

(event `/Game/Blueprints/Interfaces/BPI_InteractComponent.AddInteractableActor`
  (params (InteractableActor :type "Actor Object Reference"))
  ;[0.9115 0 0.832 0.5] Interaction System
  ;;[1 0.01123 0 0.5] Update Interactable list
  (`KismetArrayLibrary.Array_Add` (`self.InteractableItems`) InteractableActor))

(event `/Game/Blueprints/Interfaces/BPI_InteractComponent.RemoveInteractableActor`
  (params (InteractableActor :type "Actor Object Reference"))
  ;[0.9115 0 0.832 0.5] Interaction System
  ;;[1 0.01123 0 0.5] Update Interactable list
  (`KismetArrayLibrary.Array_RemoveItem` (`self.InteractableItems`) InteractableActor))

(event `/Game/Blueprints/Interfaces/BPI_PlayerController.AddMappingContext`
  (params (IMC :type "/Game/Blueprints/Enum/EPlayerMappingContext Enum" :default "NewEnumerator0"))
  ; IMC
  (bind _asplayer_controller (cast `PlayerController` (`self.GetController`)))
  (bind _returnvalue (pcsubsystem `EnhancedInputLocalPlayerSubsystem` _asplayer_controller))
  (`/Engine/EditorBlueprintResources/StandardMacros.IsValid` _returnvalue
    (:`Is Valid`
      (`EnhancedInputSubsystemInterface.AddMappingContext` _returnvalue (select `/Game/Blueprints/Enum/EPlayerMappingContext` IMC :`NewEnumerator0` "/Game/ThirdPerson/Input/IMC_Default.IMC_Default" :`NewEnumerator1` "/Game/ThirdPerson/Input/IMC_FightMode.IMC_FightMode" :!type "InputMappingContext Object Reference") 0 (struct)))))

(event `self.ReceiveBeginPlay`
  (`parent.ReceiveBeginPlay`)
  (add `/Game/Blueprints/Component/AC_Stats.Died` (`self.StatComponent`) (delegate `ManageDead`)))

(event `ManageDead`
  (`KismetSystemLibrary.PrintString` "Muerto!"))

(event `EnhancedInput|/Game/ThirdPerson/Input/Actions/IA_LightPunch`
  (params (ActionValue :type Boolean) (ElapsedSeconds :type "Float (double-precision)") (TriggeredSeconds :type "Float (double-precision)") (InputAction :type "InputAction Object Reference" :default "/Game/ThirdPerson/Input/Actions/IA_LightPunch.IA_LightPunch"))
  (:`Started`
    (if (`self.CanAttack`)
      (`|PlayMontage` (`self.Mesh`) "/Game/Models/NewAnimations/MannyPunching_Montage.MannyPunching_Montage" 1.0 0.0 (`KismetStringLibrary.Conv_StringToName` (`KismetStringLibrary.Conv_IntToString` (`self.ComboString`)))
        (:`OnCompleted`
          (set `self.ComboString` (mod (+ (`self.ComboString`) 1) 2)))))))

(event `/Game/Blueprints/Interfaces/BPI_PlayerController.SetCanAttack`
  (params (CanAttack :type Boolean))
  (set `self.CanAttack` CanAttack))

(event `/Game/Blueprints/Interfaces/BPI_PlayerController.RemoveMappingContext`
  (params (IMC :type "/Game/Blueprints/Enum/EPlayerMappingContext Enum" :default "NewEnumerator0"))
  ; IMC
  (bind _asplayer_controller (cast `PlayerController` (`self.GetController`)))
  (bind _returnvalue (pcsubsystem `EnhancedInputLocalPlayerSubsystem` _asplayer_controller))
  (`/Engine/EditorBlueprintResources/StandardMacros.IsValid` _returnvalue
    (:`Is Valid`
      (`EnhancedInputSubsystemInterface.RemoveMappingContext` _returnvalue (select `/Game/Blueprints/Enum/EPlayerMappingContext` IMC :`NewEnumerator0` "/Game/ThirdPerson/Input/IMC_Default.IMC_Default" :`NewEnumerator1` "/Game/ThirdPerson/Input/IMC_FightMode.IMC_FightMode" :!type "InputMappingContext Object Reference") (struct)))))

(event `self.Left.OnComponentBeginOverlap`
  (params (OverlappedComponent :type "PrimitiveComponent Object Reference") (OtherActor :type "Actor Object Reference") (OtherComp :type "PrimitiveComponent Object Reference") (OtherBodyIndex :type Integer) (bFromSweep :type Boolean) (SweepResult :type "HitResult Structure (by ref)"))
  (`KismetSystemLibrary.PrintString` (`KismetStringLibrary.Concat_StrStr` "Golpeo a: " (`KismetSystemLibrary.GetDisplayName` OtherActor))))

(event `self.Right.OnComponentBeginOverlap`
  (params (OverlappedComponent :type "PrimitiveComponent Object Reference") (OtherActor :type "Actor Object Reference") (OtherComp :type "PrimitiveComponent Object Reference") (OtherBodyIndex :type Integer) (bFromSweep :type Boolean) (SweepResult :type "HitResult Structure (by ref)"))
  (`KismetSystemLibrary.PrintString` (`KismetStringLibrary.Concat_StrStr` "Golpeo a: " (`KismetSystemLibrary.GetDisplayName` OtherActor))))

(event `/Game/Blueprints/Interfaces/BPI_PlayerController.SetCollision`
  (params (CollisionEnabled :type Boolean))
  (if (`self.CanAttack`)
    (if (== (`self.ComboString`) 0)
      (`PrimitiveComponent.SetCollisionEnabled` (`self.Right`) "QueryAndPhysics")
      (else
        (`PrimitiveComponent.SetCollisionEnabled` (`self.Left`) "QueryAndPhysics")))
    (else
      (`PrimitiveComponent.SetCollisionEnabled` (`self.Right`) "NoCollision")
      (`PrimitiveComponent.SetCollisionEnabled` (`self.Left`) "NoCollision"))))

(fn `UserConstructionScript`
  (`parent.UserConstructionScript`))
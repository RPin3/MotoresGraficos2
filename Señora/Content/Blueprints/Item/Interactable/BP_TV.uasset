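; BP_TV is an interactable TV actor that switches a CRT effect on and off.
; Each Interact event flips the CRTon flag and shows or hides the PostProcess component to match.
; The construction script only calls its parent, and BeginPlay, overlap and Tick are disabled stubs.
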(event `/Game/Blueprints/Interfaces/BPI_Interactable.Interact`
  (params (CharReference :type "Actor Object Reference"))
  (if (`self.CRTon`)
    (`SceneComponent.SetVisibility` (`self.PostProcess`) false false)
    (set `self.CRTon` false)
    (else
      (`SceneComponent.SetVisibility` (`self.PostProcess`) true false)
      (set `self.CRTon` true))))

(fn `UserConstructionScript`
  (`parent.UserConstructionScript`))
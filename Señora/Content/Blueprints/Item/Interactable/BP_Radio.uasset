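; BP_Radio is an interactable radio item that plays a random song each time it is used.
; Interact stops the Audio component, picks one of the first three entries in the Canciones array at random, assigns it as the sound and plays it from the start.
; The random range is hardcoded rather than taken from the array length, and the same song can repeat.
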(event `/Game/Blueprints/Interfaces/BPI_Interactable.Interact`
  (params (CharReference :type "Actor Object Reference"))
  (`AudioComponent.Stop` (`self.Audio`))
  (bind _output_get (set `self.SongIndex` (`KismetMathLibrary.RandomInteger` 3)))
  (`AudioComponent.SetSound` (`self.Audio`) (`|GetArrayItem` (`self.Canciones`) _output_get))
  (`AudioComponent.Play` (`self.Audio`) 0.0))

(fn `UserConstructionScript`
  (`parent.UserConstructionScript`))
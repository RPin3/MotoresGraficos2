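; BP_Paint is an interactable item that changes the material on its mesh each time it is interacted with.
; The Interact event advances MaterialIndex, wrapping to zero at a hard-coded limit that gives a three-step cycle.
; It then applies the matching MaterialArrays entry to the first material slot of ItemMesh.
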(event `/Game/Blueprints/Interfaces/BPI_Interactable.Interact`
  (params (CharReference :type "Actor Object Reference"))
  (if (>= (`self.MaterialIndex`) 2)
    (bind _output_get (set `self.MaterialIndex` 0))
    (`PrimitiveComponent.SetMaterial` (`self.ItemMesh`) 0 (`|GetArrayItem` (`self.MaterialArrays`) _output_get))
    (else
      (bind _result (`/Engine/EditorBlueprintResources/StandardMacros.IncrementInt` (`self.MaterialIndex`))
        (:`  `
          (bind _output_get_2 (set `self.MaterialIndex` _result))
          (`PrimitiveComponent.SetMaterial` (`self.ItemMesh`) 0 (`|GetArrayItem` (`self.MaterialArrays`) _output_get_2)))))))

(fn `UserConstructionScript`
  (`parent.UserConstructionScript`))
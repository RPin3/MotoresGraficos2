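; BP_Light is an interactable light actor that switches on and off when interacted with.
; Its Interact event checks the IsOn flag, toggles the PointLight component's visibility to the opposite state and updates the flag.
; BeginPlay, overlap and Tick are unused, and the construction script only calls its parent.
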(event `/Game/Blueprints/Interfaces/BPI_Interactable.Interact`
  (params (CharReference :type "Actor Object Reference"))
  (if (`self.isOn`)
    (`SceneComponent.SetVisibility` (`self.PointLight`) false false)
    (set `self.isOn` false)
    (else
      (`SceneComponent.SetVisibility` (`self.PointLight`) true false)
      (set `self.isOn` true))))

(fn `UserConstructionScript`
  (`parent.UserConstructionScript`))
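; BP_Door is an interactable door that swings open and closed when a character interacts with it.
; Interact uses a dot product between the character-to-door direction and the root's forward vector to decide which side the character is on.
; A FlipFlop alternates playing and reversing the DoorOpen timeline, which lerps the door's yaw to plus or minus 90 degrees based on that side.
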(event `/Game/Blueprints/Interfaces/BPI_Interactable.Interact`
  (params (CharReference :type "Actor Object Reference"))
  (set `self.IsOutside` (> (`KismetMathLibrary.Dot_VectorVector` (`KismetMathLibrary.GetDirectionUnitVector` (`self.K2_GetActorLocation` CharReference) (`self.K2_GetActorLocation`)) (`SceneComponent.GetForwardVector` (`self.DefaultSceneRoot`))) 0.0))
  (`/Engine/EditorBlueprintResources/StandardMacros.FlipFlop`
    (:`A`
      (bind (_direction _delta_open) (`Timeline|DoorOpen` :!label _label)
        (:`Update`
          (`SceneComponent.K2_SetRelativeRotation` (`self.Door`) (`KismetMathLibrary.MakeRotator` 0.0 0.0 (`KismetMathLibrary.Lerp` 0.0 (`KismetMathLibrary.SelectFloat` 90.0 -90.0 (`self.IsOutside`)) _delta_open)) false false))))
    (:`B`
      (goto _label :!via `Reverse`))))

(fn `UserConstructionScript`
  (`parent.UserConstructionScript`))
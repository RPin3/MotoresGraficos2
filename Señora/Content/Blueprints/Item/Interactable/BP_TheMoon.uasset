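; BP_TheMoon is an interactable moon item that toggles a "Dark Hour" mode on and off.
; Each Interact call checks the DarkHour flag, then flips it.
; Turning it on swaps the mesh to an instance moon material, shows the post-process component and plays the Masteroftartarus sound.
; Turning it off restores the base moon material, hides the post-process and stops the audio.
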(event `/Game/Blueprints/Interfaces/BPI_Interactable.Interact`
  (params (CharReference :type "Actor Object Reference"))
  (if (`self.DarkHour`)
    (`PrimitiveComponent.SetMaterial` (`self.ItemMesh`) 0 "/Game/Blueprints/Item/Interactable/Materials/M_Moon.M_Moon")
    (`SceneComponent.SetVisibility` (`self.PostProcess`) false false)
    (`AudioComponent.Stop` (`self.Audio`))
    (set `self.DarkHour` false)
    (else
      (`PrimitiveComponent.SetMaterial` (`self.ItemMesh`) 0 "/Game/Blueprints/Item/Interactable/Materials/M_Moon_Inst.M_Moon_Inst")
      (`SceneComponent.SetVisibility` (`self.PostProcess`) true false)
      (`AudioComponent.SetSound` (`self.Audio`) "/Game/Blueprints/Item/Interactable/Radio/master-of-tartarus.master-of-tartarus")
      (`AudioComponent.Play` (`self.Audio`) 0.0)
      (set `self.DarkHour` true))))

(fn `UserConstructionScript`
  (`parent.UserConstructionScript`))
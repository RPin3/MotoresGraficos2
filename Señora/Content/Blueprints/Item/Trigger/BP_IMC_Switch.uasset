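; BP_IMC_Switch is a trigger item that switches input mapping contexts on whatever actor triggers it.
; Its Trigger event sends an add message to the Causer for each entry in IMCToAdd, then a remove message for each entry in IMCToRemove.
; The mapping changes themselves are left to the Causer, and the Blueprint has no active overlap or tick logic of its own.
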(event `self.Trigger`
  (params (Causer :type "Actor Object Reference"))
  (for _array_element (`self.IMCToAdd`)
    (message `/Game/Blueprints/Interfaces/BPI_PlayerController.AddMappingContext` Causer _array_element))
  (for _array_element_2 (`self.IMCToRemove`)
    (message `/Game/Blueprints/Interfaces/BPI_PlayerController.RemoveMappingContext` Causer _array_element_2)))

(fn `UserConstructionScript`
  (`parent.UserConstructionScript`))
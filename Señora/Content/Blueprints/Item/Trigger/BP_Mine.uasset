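; BP_Mine is a triggerable mine item that explodes and deals area damage.
; Its Trigger event spawns an explosion emitter at the actor's location, then runs a sphere trace on the Pawn profile around it.
; Each hit actor receives environmental damage equal to BaseDamage, with no falloff or deduplication of hits, and the mine then destroys itself.
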(event `self.Trigger`
  (params (Causer :type "Actor Object Reference"))
  (bind _returnvalue (`self.K2_GetActorLocation`))
  (`GameplayStatics.SpawnEmitterAtLocation` "/Game/StarterContent/Particles/P_Explosion.P_Explosion" (`self.K2_GetActorLocation`))
  (bind _outhits (`KismetSystemLibrary.SphereTraceMultiByProfile` _returnvalue _returnvalue 1000.0 "Pawn"))
  (for _array_element _outhits
    (`GameplayStatics.ApplyDamage` (`.HitActor` (`GameplayStatics.BreakHitResult` _array_element)) (`self.Base Damage`) null self "/Engine/EngineDamageTypes/DmgTypeBP_Environmental.DmgTypeBP_Environmental_C"))
  (`self.K2_DestroyActor`))

(fn `UserConstructionScript`
  (`parent.UserConstructionScript`))